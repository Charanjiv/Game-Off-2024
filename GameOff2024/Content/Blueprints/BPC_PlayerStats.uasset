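; Player stats component that tracks health and stamina for the BP_ThirdPersonCharacter that owns it.
; Health changes, with healing capped at the maximum, push directly to the character's HUD progress bar and text.
; Stamina changes skip the HUD, and both decrease functions return whether the value is depleted.
; IncreaseMaxStamina sets the maximum to zero, as its addition is left unconnected.
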(event EventBeginPlay
  (bind _asbp_third_person_character (Utilities|Casting|CastToBP_ThirdPersonCharacter (Components|GetOwner)))
  (Variables|Default|SetPlayerCharacter _asbp_third_person_character))

(event EventTick
  (params (DeltaSeconds :type Float%20%28single-precision%29)))

(fn DecreaseHealth
  (params (Damage :type Float%20%28double-precision%29))
  (bind _playercharacter (Variables|Default|GetPlayerCharacter))
  (bind _hudwidget (Variables|/Game/ThirdPerson/Blueprints/BP_ThirdPersonCharacter.BP_ThirdPersonCharacter_C|GetHUDWidget _playercharacter))
  (bind _output_get (Variables|Health|SetCurrentHealth (- (Variables|Health|GetCurrentHealth) Damage)))
  (Progress|SetPercent (Variables|/Game/UI/WBP_HUD.WBP_HUD_C|GetProgressBar_Health _hudwidget) (/ _output_get (Variables|Health|GetMaxHealth)))
  (Rendering|Components|TextRender|SetText (Variables|/Game/UI/WBP_HUD.WBP_HUD_C|GetText_Health _hudwidget) (Utilities|Text|ToText(Float) (Variables|Health|GetCurrentHealth) "HalfToEven"))
  (if (<= (Variables|Health|GetCurrentHealth) 0.0)
    (return true)
    (else
      (return false))))

(fn IncreaseMaxHealth
  (params (IncrementHealth :type Float%20%28double-precision%29))
  (bind _playercharacter (Variables|Default|GetPlayerCharacter))
  (bind _hudwidget (Variables|/Game/ThirdPerson/Blueprints/BP_ThirdPersonCharacter.BP_ThirdPersonCharacter_C|GetHUDWidget _playercharacter))
  (Variables|Health|SetMaxHealth (+ (Variables|Health|GetMaxHealth) IncrementHealth))
  (Progress|SetPercent (Variables|/Game/UI/WBP_HUD.WBP_HUD_C|GetProgressBar_Health _hudwidget) (/ (Variables|Health|GetCurrentHealth) (Variables|Health|GetMaxHealth)))
  (Rendering|Components|TextRender|SetText (Variables|/Game/UI/WBP_HUD.WBP_HUD_C|GetText_Health _hudwidget) (Utilities|Text|ToText(Float) (Variables|Health|GetCurrentHealth) "HalfToEven")))

(fn DecreaseStamina
  (params (StaminaDepleted :type Float%20%28double-precision%29))
  (Variables|Stamina|SetCurrentStamina (- (Variables|Stamina|GetCurrentStamina) StaminaDepleted))
  (if (<= (Variables|Stamina|GetCurrentStamina) 0.0)
    (return true)
    (else
      (return false))))

(fn IncreaseMaxStamina
  (params (AddedStamina :type Float%20%28double-precision%29))
  (Variables|Stamina|SetMaxStamina 0.0))

(fn IncreaseHealth
  (params (AddedHealth :type Float%20%28double-precision%29))
  (bind _playercharacter (Variables|Default|GetPlayerCharacter))
  (bind _hudwidget (Variables|/Game/ThirdPerson/Blueprints/BP_ThirdPersonCharacter.BP_ThirdPersonCharacter_C|GetHUDWidget _playercharacter))
  (Variables|Health|SetCurrentHealth (+ (Variables|Health|GetCurrentHealth) AddedHealth))
  (if (> (Variables|Health|GetCurrentHealth) (Variables|Health|GetMaxHealth))
    (Variables|Health|SetCurrentHealth (Variables|Health|GetMaxHealth)))
  (Progress|SetPercent (Variables|/Game/UI/WBP_HUD.WBP_HUD_C|GetProgressBar_Health _hudwidget) (/ (Variables|Health|GetCurrentHealth) (Variables|Health|GetMaxHealth)))
  (Rendering|Components|TextRender|SetText (Variables|/Game/UI/WBP_HUD.WBP_HUD_C|GetText_Health _hudwidget) (Utilities|Text|ToText(Float) (Variables|Health|GetCurrentHealth) "HalfToEven")))

(fn IncreaseStamina
  (params (AddedStamina :type Float%20%28double-precision%29))
  (Variables|Stamina|SetCurrentStamina (+ (Variables|Stamina|GetCurrentStamina) AddedStamina))
  (if (> (Variables|Stamina|GetCurrentStamina) (Variables|Stamina|GetMaxStamina))
    (Variables|Stamina|SetCurrentStamina (Variables|Stamina|GetMaxStamina))))